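; Enemy AI character with melee combos, health, ragdoll death and player stealth assassination.
; Buffered attack input chains combo montages, while timer-looped weapon or single-point sphere traces damage "Damagable" actors with effects.
; Damage cancels attacks, plays a reaction, launches it along the player's facing and calls Kill based on BPCStats.
; Camera-facing widgets show stats, an overlap-driven assassinate prompt and a toggled investigate indicator; StealthAssassinate returns an alignment transform and triggers delayed death.
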(event `self.ReceiveBeginPlay`
  (bind _aswb_dummy_stats (cast `/Game/UI/WB_DummyStats` (`WidgetComponent.GetUserWidgetObject` (`self.StatsWidget`))))
  (set `/Game/UI/WB_DummyStats.Stats` (`self.BPC_Stats`) _aswb_dummy_stats))

(event `self.ReceiveTick`
  (params (DeltaSeconds :type "Float (single-precision)"))
  (bind _returnvalue (`KismetMathLibrary.FindLookAtRotation` (`SceneComponent.K2_GetComponentLocation` (`self.AssassinateWidget`)) (`SceneComponent.K2_GetComponentLocation` (`PlayerCameraManager.TransformComponent` (`GameplayStatics.GetPlayerCameraManager` 0)))))
  ;[0.05098 0.05098 0.05098] Rotate UI
  (`SceneComponent.K2_SetWorldRotation` (`self.AssassinateWidget`) _returnvalue false false)
  (`SceneComponent.K2_SetWorldRotation` (`self.InvestigateWidget`) _returnvalue false false)
  (`SceneComponent.K2_SetWorldRotation` (`self.StatsWidget`) _returnvalue false false))

(event `Kill`
  (params (`Physics Delay` :type "Float (double-precision)" :default 2.5) (`Audio Delay` :type "Float (double-precision)" :default 1.5))
  (bind _mesh (`self.Mesh`))
  ;[0.05098 0.05098 0.05098] Death
  (`|ExecutionSequence`
    (:`then_0`
      (`KismetSystemLibrary.Delay` `Physics Delay`)
      (`PrimitiveComponent.SetCollisionObjectType` _mesh "ECC_PhysicsBody")
      (`PrimitiveComponent.SetSimulatePhysics` _mesh true))
    (:`then_1`
      (`KismetSystemLibrary.Delay` `Audio Delay`)
      (`GameplayStatics.PlaySoundAtLocation` "/Game/Audio/Combat/Hit/SC_Death.SC_Death" (`self.K2_GetActorLocation`) (struct) 1.0 1.0 0.0 "/Game/Audio/SA_Player.SA_Player" null null null)
      (`CharacterMovementComponent.SetMovementMode` (`self.CharacterMovement`) "MOVE_None" 0))))

(event `self.AssassinationRadius.OnComponentBeginOverlap`
  (params (OverlappedComponent :type "PrimitiveComponent Object Reference") (OtherActor :type "Actor Object Reference") (OtherComp :type "PrimitiveComponent Object Reference") (OtherBodyIndex :type Integer) (bFromSweep :type Boolean) (SweepResult :type "HitResult Structure (by ref)"))
  ;[0.05098 0.05098 0.05098] Show/Hide Assasination UI
  (cast `/Game/Blueprints/Player/BP_ThirdPersonCharacter` OtherActor)
  (`SceneComponent.SetVisibility` (`self.AssassinateWidget`) true false))

(event `self.AssassinationRadius.OnComponentEndOverlap`
  (params (OverlappedComponent :type "PrimitiveComponent Object Reference") (OtherActor :type "Actor Object Reference") (OtherComp :type "PrimitiveComponent Object Reference") (OtherBodyIndex :type Integer))
  ;[0.05098 0.05098 0.05098] Show/Hide Assasination UI
  (cast `/Game/Blueprints/Player/BP_ThirdPersonCharacter` OtherActor)
  (`SceneComponent.SetVisibility` (`self.AssassinateWidget`) false false))

(event `self.ReceiveAnyDamage`
  (params (Damage :type "Float (single-precision)") (DamageType :type "DamageType Object Reference") (InstigatedBy :type "Controller Object Reference") (DamageCauser :type "Actor Object Reference"))
  ;[0.05098 0.05098 0.05098] Damage
  (`self.StopAttack`)
  (`self.PlayAnimMontage` (`KismetArrayLibrary.Array_Random` (`self.HitAnimations`)))
  (bind _asbp_third_person_character (cast `/Game/Blueprints/Player/BP_ThirdPersonCharacter` (`GameplayStatics.GetPlayerCharacter` 0)))
  (`self.LaunchCharacter` (* (`KismetMathLibrary.GetForwardVector` (`self.K2_GetActorRotation` _asbp_third_person_character)) 700.0))
  (`GameplayStatics.PlaySoundAtLocation` "/Game/Audio/Combat/Hit/Grunt.Grunt" (`self.K2_GetActorLocation`) (struct) 1.0 (`KismetMathLibrary.RandomFloatInRange` -1.1 1.1) 0.0 null null null null)
  (bind _isdead (`/Game/Blueprints/Player/BPC_Stats.DecreaseCurrentHealth` (`self.BPC_Stats`) Damage))
  (if _isdead
    (`self.Kill` 0.0 0.0)))

(event `Play Attack Animation`
  ;[0.05098 0.05098 0.05098] Attacks and Combos
  ;;[0.05098 0.05098 0.05098] Play Attack Animation
  (if (`KismetArrayLibrary.Array_IsValidIndex` (`self.ComboAnimations`) (`self.AttackIndex`))
    (`/Engine/EditorBlueprintResources/StandardMacros.DoOnce` false :!label _label
      (:`Completed`
        (`KismetSystemLibrary.Delay` 0.1)
        (`|PlayMontage` (`self.Mesh`) (`|GetArrayItem` (`self.ComboAnimations`) (`self.AttackIndex`)) (`self.AnimationPlayRate`)
          (:`then`
            (`/Engine/EditorBlueprintResources/StandardMacros.IncrementInt` (`self.AttackIndex`)
              (:`  `
                (goto _label :!via `Reset`)))))))))

(event `MeleeAttackCombo`
  ;[0.05098 0.05098 0.05098] Attacks and Combos
  ;;[0.05098 0.05098 0.05098] Attack Input
  (if (`self.CanAttack`)
    (`self.BeginAttack`)))

(event `BeginAttack`
  ;[0.05098 0.05098 0.05098] Attacks and Combos
  ;;[0.05098 0.05098 0.05098] Begin Attack
  (if (`self.IsAttacking`)
    (set `self.HasSavedAttack` true)
    (else
      (set `self.IsAttacking` true)
      (`self.Play Attack Animation`))))

(event `Continue Combo`
  ;[0.05098 0.05098 0.05098] Attacks and Combos
  ;;[0.05098 0.05098 0.05098] Continue Combo
  (if (`self.HasSavedAttack`)
    (set `self.HasSavedAttack` false)
    (`self.Play Attack Animation`)
    (else
      (`self.StopAttack`))))

(event `StopAttack`
  ;[0.05098 0.05098 0.05098] Attacks and Combos
  ;;[0.05098 0.05098 0.05098] Stop Combo/Attack
  (set `self.IsAttacking` false)
  (set `self.AttackIndex` 0))

(event `BeginSwordTrace`
  ;[0.05098 0.05098 0.05098] Sword Trace
  (bind _returnvalue (`KismetSystemLibrary.K2_SetTimerDelegate` (delegate `SwordTraceLoop`) 0.001 true))
  (set `self.Sword Trace Timer` _returnvalue))

(event `HandleHit`
  (params (`Hit Target` :type "Actor Object Reference") (`Hit Location` :type "Vector Structure") (`Hit Rotation` :type "Rotator Structure"))
  ;[0.05098 0.05098 0.05098] HandleHit
  (if (`self.ActorHasTag` `Hit Target` "Damagable")
    (`/Engine/EditorBlueprintResources/StandardMacros.DoOnce` false :!label _label_2
      (:`Completed`
        (`GameplayStatics.ApplyDamage` `Hit Target` 10.0)
        (`GameplayStatics.PlayWorldCameraShake` "/Game/Blueprints/Combat/BP_HitCameraShake.BP_HitCameraShake_C" `Hit Location` 0.0 2000.0)
        (`self.PlayHitAudio`)
        (`GameplayStatics.SpawnEmitterAtLocation` "/Game/Particles/Blood/P_Blood_Splat_Cone.P_Blood_Splat_Cone" `Hit Location` `Hit Rotation` (0.4 0.4 0.4) true "AutoRelease")
        (`KismetSystemLibrary.Delay` 0.5)
        (goto _label_2 :!via `Reset`)))))

(event `SwordTraceLoop`
  ;[0.05098 0.05098 0.05098] Sword Trace
  (bind (_outhit _returnvalue) (`KismetSystemLibrary.SphereTraceSingle` (`SceneComponent.K2_GetComponentLocation` (`self.WeaponTipPoint`)) (`SceneComponent.K2_GetComponentLocation` (`self.WeaponBasePoint`)) 12.0 "TraceTypeQuery1"))
  (if _returnvalue
    (bind (_bblockinghit _binitialoverlap _time _distance _location _impactpoint _normal _impactnormal _physmat _hitactor) (`GameplayStatics.BreakHitResult` _outhit))
    (`self.HandleHit` _hitactor _location (`KismetMathLibrary.MakeRotFromXY` _normal _normal))))

(event `PlayHitAudio`
  ;[0.05098 0.05098 0.05098] HandleHit
  ;;[0.05098 0.05098 0.05098] Play Hit Audio
  (`GameplayStatics.PlaySoundAtLocation` "/Game/Audio/Combat/Attack/MS_SwordHit.MS_SwordHit" (`self.K2_GetActorLocation` (`self.GetOwner`)) (struct) 1.0 1.0 0.0 "/Game/Audio/SA_Player.SA_Player" null null null))

(event `StopSwordTrace`
  ;[0.05098 0.05098 0.05098] Sword Trace
  (`KismetSystemLibrary.K2_ClearAndInvalidateTimerHandle` (`self.Sword Trace Timer`)))

(event `HitTrace`
  (bind _returnvalue (`SceneComponent.K2_GetComponentLocation` (`self.HitTraceArrow`)))
  ;[0.05098 0.05098 0.05098] Hit Trace
  (bind (_outhit _returnvalue_2) (`KismetSystemLibrary.SphereTraceSingle` _returnvalue _returnvalue 25.0 "TraceTypeQuery1"))
  (if _returnvalue_2
    (bind (_bblockinghit _binitialoverlap _time _distance _location _impactpoint _normal _impactnormal _physmat _hitactor) (`GameplayStatics.BreakHitResult` _outhit))
    (`self.HandleHit` _hitactor _location (`KismetMathLibrary.MakeRotFromXY` _normal _normal))))

(event `EnableInvestigateUI`
  (bind _isa (`/Engine/EditorBlueprintResources/StandardMacros.FlipFlop`)
    (:`A`
      _)
    (:`B`
      _))
  (`SceneComponent.SetVisibility` (`self.InvestigateWidget`) _isa false))

(fn `Attack`
  (returns (AnimationDuration :type "Float (double-precision)"))
  (`self.MeleeAttackCombo`)
  (return 0.0))

(fn `StealthAssassinate`
  (returns (Location :type "Vector Structure") (Rotation :type "Rotator Structure"))
  (`self.PlayAnimMontage` "/Game/Characters/RPG_Character/Animations/Assassinations/StealthKnifeAttack_Victim_Montage.StealthKnifeAttack_Victim_Montage")
  (`self.Kill` 2.5)
  (`SceneComponent.SetVisibility` (`self.AssassinateWidget`) false false)
  (return (`SceneComponent.K2_GetComponentLocation` (`self.Assassinate REF`)) (`self.K2_GetActorRotation`)))

(fn `UserConstructionScript`)