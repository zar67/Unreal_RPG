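; Generic AI controller that runs the BT_AI behavior tree and feeds it sight and hearing results through the Blackboard.
; Each perception update goes to both handlers: successful sight sets TargetActor, and any other update clears it.
; InvestigationLocation takes the stimulus location on every update, whatever the sense or result.
; Successful hearing also enables the investigate UI on the controlled BP_AI pawn.
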(event `self.ReceiveBeginPlay`
  (`self.RunBehaviorTree` "/Game/AI/BT_AI.BT_AI"))

(event `self.AIPerception.OnTargetPerceptionUpdated`
  (params (Actor :type "Actor Object Reference") (Stimulus :type "AIStimulus Structure"))
  ;[0.05098 0.05098 0.05098] Detect Target Actor
  (`self.DetectSeenTarget` Actor Stimulus)
  (`self.DetectHeardTarget` Actor Stimulus))

(event `DetectSeenTarget`
  (params (Actor :type "Actor Object Reference") (Stimulus :type "AIStimulus Structure"))
  (bind _returnvalue (`AIBlueprintHelperLibrary.GetBlackboard` null))
  ;[0.05098 0.05098 0.05098] Detect Target Actor
  (bind _returnvalue_2 (`AIPerceptionSystem.GetSenseClassForStimulus` Stimulus))
  (if (and (== _returnvalue_2 "/Script/AIModule.AISense_Sight") (`.bSuccessfullySensed` (break `AIStimulus` Stimulus)))
    (`BlackboardComponent.SetValueAsObject` _returnvalue "TargetActor" Actor)
    (else
      (`BlackboardComponent.SetValueAsObject` _returnvalue "TargetActor" null))))

(event `DetectHeardTarget`
  (params (Actor :type "Actor Object Reference") (Stimulus :type "AIStimulus Structure"))
  (bind (_age _expirationage _strength _stimuluslocation _receiverlocation _tag _bsuccessfullysensed) (break `AIStimulus` Stimulus))
  (bind _returnvalue (`AIBlueprintHelperLibrary.GetBlackboard` null))
  ;[0.05098 0.05098 0.05098] Detect Target Actor
  (bind _returnvalue_2 (`AIPerceptionSystem.GetSenseClassForStimulus` Stimulus))
  (if (and (== _returnvalue_2 "/Script/AIModule.AISense_Hearing") _bsuccessfullysensed)
    (`BlackboardComponent.SetValueAsVector` _returnvalue "InvestigationLocation" _stimuluslocation)
    (bind _asbp_ai (cast `/Game/AI/BP_AI` (`self.K2_GetPawn`)))
    (`/Game/AI/BP_AI.EnableInvestigateUI` _asbp_ai)
    (else
      (`BlackboardComponent.SetValueAsVector` _returnvalue "InvestigationLocation" _stimuluslocation))))

(fn `UserConstructionScript`)