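; AI controller for boss enemies that runs the boss behavior tree and manages the boss health bar UI.
; BeginPlay starts BT_AI_Boss.
; ActivateBossCombat creates a WB_BossHealth widget, adds it to the viewport and hands it the stats component of the controlled BP_AI pawn.
; DeactivateBossCombat removes the widget and clears its reference.
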(event `self.ReceiveBeginPlay`
  (`self.RunBehaviorTree` "/Game/AI/Boss/BT_AI_Boss.BT_AI_Boss"))

(event `ActivateBossCombat`
  (bind _returnvalue (`|CreateWidget` "/Game/UI/WB_BossHealth.WB_BossHealth_C"))
  (bind _output_get (set `self.Boss Health Bar` _returnvalue))
  (`UserWidget.AddToViewport` _output_get 0)
  (bind _asbp_ai (cast `/Game/AI/BP_AI` (`self.K2_GetPawn`)))
  (set `/Game/UI/WB_BossHealth.Stats` (`/Game/AI/BP_AI.BPC_Stats` _asbp_ai) (`self.Boss Health Bar`)))

(event `DeactivateBossCombat`
  (`Widget.RemoveFromParent` (`self.Boss Health Bar`))
  (set `self.Boss Health Bar` null))

(fn `UserConstructionScript`
  (`parent.UserConstructionScript`))