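; Player stats component that tracks health, stamina, XP and level.
; Functions raise or lower health and stamina, clamped between zero and their maximums, and return whether a limit is reached, with health loss also setting IsDead.
; Raising a maximum adds the same amount to the current value.
; XP gains loop through level-ups, carrying over the remainder, raising the next threshold linearly and playing two 2D sounds per level.
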(fn `DecreaseCurrentHealth`
  (params (DecreaseAmount :type "Float (double-precision)"))
  (returns (IsDead :type Boolean))
  (bind _output_get (set `self.CurrentHealth` (`KismetMathLibrary.FClamp` (- (`self.CurrentHealth`) DecreaseAmount) 0.0 (`self.MaxHealth`))))
  (bind _output_get_2 (set `self.IsDead` (<= _output_get 0.0)))
  (return _output_get_2))

(fn `DecreaseCurrentStamina`
  (params (DecreaseAmount :type "Float (double-precision)"))
  (returns (IsDrained :type Boolean))
  (bind _output_get (set `self.Current Stamina` (`KismetMathLibrary.FClamp` (- (`self.Current Stamina`) DecreaseAmount) 0.0 (`self.MaxStamina`))))
  (return (<= _output_get 0.0)))

(fn `IncreaseCurrentHealth`
  (params (IncreaseAmount :type "Float (double-precision)"))
  (returns (IsMaxHealth :type Boolean))
  (bind _output_get (set `self.CurrentHealth` (`KismetMathLibrary.FClamp` (+ IncreaseAmount (`self.CurrentHealth`)) 0.0 (`self.MaxHealth`))))
  (return (>= _output_get (`self.MaxHealth`))))

(fn `IncreaseCurrentStamina`
  (params (IncreaseAmount :type "Float (double-precision)"))
  (returns (IsMaxStamina :type Boolean))
  (bind _output_get (set `self.Current Stamina` (`KismetMathLibrary.FClamp` (+ IncreaseAmount (`self.Current Stamina`)) 0.0 (`self.MaxStamina`))))
  (return (>= _output_get (`self.MaxStamina`))))

(fn `IncreaseMaxHealth`
  (params (IncreaseAmount :type "Float (double-precision)"))
  (set `self.MaxHealth` (+ IncreaseAmount (`self.MaxHealth`)))
  (set `self.CurrentHealth` (+ IncreaseAmount (`self.CurrentHealth`))))

(fn `IncreaseMaxStamina`
  (params (IncreaseAmount :type "Float (double-precision)"))
  (set `self.MaxStamina` (+ IncreaseAmount (`self.MaxStamina`)))
  (set `self.Current Stamina` (+ IncreaseAmount (`self.Current Stamina`))))

(fn `IncreaseXP`
  (params (IncreaseAmount :type "Float (double-precision)"))
  (returns (NewLevel :type Integer))
  (set `self.CurrentXP` (+ IncreaseAmount (`self.CurrentXP`)))
  (while (>= (`self.CurrentXP`) (`self.MaxXP`))
    (set `self.CurrentLevel` (+ (`self.CurrentLevel`) 1))
    (`GameplayStatics.PlaySound2D` "/Game/Audio/UI/LevelUp1.LevelUp1" 1.0 1.0 0.0 null null)
    (`GameplayStatics.PlaySound2D` "/Game/Audio/UI/LevelUp2.LevelUp2" 1.0 1.0 0.0 null null)
    (set `self.CurrentXP` (- (`self.CurrentXP`) (`self.MaxXP`)))
    (set `self.MaxXP` (+ (`self.MaxXP`) 150.0)))
  (return (`self.CurrentLevel`)))