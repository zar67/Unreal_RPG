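; Component that gives BP_ThirdPersonCharacter a melee combo attack with sword and point hit detection.
; Attack input starts or buffers the next montage in ComboAnimations, and ContinueCombo plays the saved attack or resets the chain.
; A looping timer sphere-traces between sword tip and base, while HitTrace does a single trace at a character point.
; Both feed HandleHit, which damages "Damagable" actors with camera shake and sound, gated by a short cooldown.
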(event `self.ReceiveBeginPlay`
  (bind _asbp_third_person_character (cast `/Game/ThirdPerson/Blueprints/BP_ThirdPersonCharacter` (`self.GetOwner`)))
  (set `self.CharacterBP` _asbp_third_person_character)
  (set `self.CharacterMesh` (`Character.Mesh` _asbp_third_person_character)))

(event `Play Attack Animation`
  ;[0.05098 0.05098 0.05098] Attacks and Combos
  ;;[0.05098 0.05098 0.05098] Play Attack Animation
  (if (`KismetArrayLibrary.Array_IsValidIndex` (`self.ComboAnimations`) (`self.AttackIndex`))
    (`/Engine/EditorBlueprintResources/StandardMacros.DoOnce` false :!label _label
      (:`Completed`
        (`KismetSystemLibrary.Delay` 0.1)
        (`|PlayMontage` (`self.CharacterMesh`) (`|GetArrayItem` (`self.ComboAnimations`) (`self.AttackIndex`))
          (:`then`
            (`/Engine/EditorBlueprintResources/StandardMacros.IncrementInt` (`self.AttackIndex`)
              (:`  `
                (goto _label :!via `Reset`)))))))))

(event `EnhancedInput|/Game/ThirdPerson/Input/Actions/IA_Attack`
  (params (ActionValue :type Boolean) (ElapsedSeconds :type "Float (double-precision)") (TriggeredSeconds :type "Float (double-precision)") (InputAction :type "InputAction Object Reference" :default "/Game/ThirdPerson/Input/Actions/IA_Attack.IA_Attack"))
  ;[0.05098 0.05098 0.05098] Attacks and Combos
  ;;[0.05098 0.05098 0.05098] Attack Input
  (:`Started`
    (if (`self.CanAttack`)
      (`self.BeginAttack`))))

(event `BeginAttack`
  ;[0.05098 0.05098 0.05098] Attacks and Combos
  ;;[0.05098 0.05098 0.05098] Begin Attack
  (if (`self.IsAttacking`)
    (set `self.HasSavedAttack` true)
    (else
      (set `self.IsAttacking` true)
      (`self.Play Attack Animation`))))

(event `Continue Combo`
  ;[0.05098 0.05098 0.05098] Attacks and Combos
  ;;[0.05098 0.05098 0.05098] Continue Combo
  (if (`self.HasSavedAttack`)
    (set `self.HasSavedAttack` false)
    (`self.Play Attack Animation`)
    (else
      (`self.StopAttack`))))

(event `StopAttack`
  ;[0.05098 0.05098 0.05098] Attacks and Combos
  ;;[0.05098 0.05098 0.05098] Stop Combo/Attack
  (set `self.IsAttacking` false)
  (set `self.AttackIndex` 0))

(event `BeginSwordTrace`
  ;[0.05098 0.05098 0.05098] Sword Trace
  (bind _returnvalue (`KismetSystemLibrary.K2_SetTimerDelegate` (delegate `SwordTraceLoop`) 0.001 true))
  (set `self.SwordTraceTimer` _returnvalue))

(event `HandleHit`
  (params (`Hit Target` :type "Actor Object Reference") (`Hit Location` :type "Vector Structure"))
  ;[0.05098 0.05098 0.05098] HandleHit
  (if (`Actor.ActorHasTag` `Hit Target` "Damagable")
    (`/Engine/EditorBlueprintResources/StandardMacros.DoOnce` false :!label _label_2
      (:`Completed`
        (`GameplayStatics.ApplyDamage` `Hit Target` 10.0)
        (`GameplayStatics.PlayWorldCameraShake` "/Game/Blueprints/Combat/BP_HitCameraShake.BP_HitCameraShake_C" `Hit Location` 0.0 2000.0)
        (`self.PlayHitAudio`)
        (`KismetSystemLibrary.Delay` 0.5)
        (goto _label_2 :!via `Reset`)))))

(event `SwordTraceLoop`
  (bind _characterbp (`self.CharacterBP`))
  ;[0.05098 0.05098 0.05098] Sword Trace
  (bind (_outhit _returnvalue) (`KismetSystemLibrary.SphereTraceSingle` (`SceneComponent.K2_GetComponentLocation` (`/Game/ThirdPerson/Blueprints/BP_ThirdPersonCharacter.SwordTipPoint` _characterbp)) (`SceneComponent.K2_GetComponentLocation` (`/Game/ThirdPerson/Blueprints/BP_ThirdPersonCharacter.SwordBasePoint` _characterbp)) 12.0 "TraceTypeQuery1"))
  (if _returnvalue
    (bind (_bblockinghit _binitialoverlap _time _distance _location _impactpoint _normal _impactnormal _physmat _hitactor) (`GameplayStatics.BreakHitResult` _outhit))
    (`self.HandleHit` _hitactor _location)))

(event `PlayHitAudio`
  ;[0.05098 0.05098 0.05098] HandleHit
  ;;[0.05098 0.05098 0.05098] Play Hit Audio
  (`GameplayStatics.PlaySoundAtLocation` "/Game/Audio/Combat/Attack/MS_SwordHit.MS_SwordHit" (`Actor.K2_GetActorLocation` (`self.GetOwner`)) (struct) 1.0 1.0 0.0 "/Game/Audio/SA_Player.SA_Player" null null null))

(event `StopSwordTrace`
  ;[0.05098 0.05098 0.05098] Sword Trace
  (`KismetSystemLibrary.K2_ClearAndInvalidateTimerHandle` (`self.SwordTraceTimer`)))

(event `HitTrace`
  (bind _returnvalue (`SceneComponent.K2_GetComponentLocation` (`/Game/ThirdPerson/Blueprints/BP_ThirdPersonCharacter.HitTrace` (`self.CharacterBP`))))
  ;[0.05098 0.05098 0.05098] Hit Trace
  (bind (_outhit _returnvalue_2) (`KismetSystemLibrary.SphereTraceSingle` _returnvalue _returnvalue 25.0 "TraceTypeQuery1"))
  (if _returnvalue_2
    (bind (_bblockinghit _binitialoverlap _time _distance _location _impactpoint _normal _impactnormal _physmat _hitactor) (`GameplayStatics.BreakHitResult` _outhit))
    (`self.HandleHit` _hitactor _location)))