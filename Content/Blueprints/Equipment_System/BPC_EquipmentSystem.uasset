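; Equipment component for the third-person character that handles weapon pickup and the equipment menu.
; On interact, a sphere trace from the follow camera finds a BP_Weapon, stores its ItemData in WeaponSlots and destroys the actor.
; The menu input toggles a lazily created, reused WB_EquipmentMenu widget, switching cursor and input mode.
; While the menu is open, character movement and attacking are disabled.
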(event `self.ReceiveBeginPlay`
  (bind _asbp_third_person_character (cast `/Game/Blueprints/Player/BP_ThirdPersonCharacter` (`self.GetOwner`)))
  (set `self.Follow Camera` (`/Game/Blueprints/Player/BP_ThirdPersonCharacter.FollowCamera` _asbp_third_person_character)))

(event `EnhancedInput|/Game/Input/Actions/IA_Interact`
  (params (ActionValue :type Boolean) (ElapsedSeconds :type "Float (double-precision)") (TriggeredSeconds :type "Float (double-precision)") (InputAction :type "InputAction Object Reference" :default "/Game/Input/Actions/IA_Interact.IA_Interact"))
  (bind _follow_camera (`self.Follow Camera`))
  (bind _returnvalue (`SceneComponent.K2_GetComponentLocation` _follow_camera))
  ;[0.05098 0.05098 0.05098] Item Interaction
  (:`Started`
    (bind _outhit (`KismetSystemLibrary.SphereTraceSingleForObjects` _returnvalue (+ _returnvalue (* (`KismetMathLibrary.GetForwardVector` (`SceneComponent.K2_GetComponentRotation` _follow_camera)) 1000.0)) 15.0 (`|MakeArray` "ObjectTypeQuery2" :!type "EObjectTypeQuery Enum")))
    (if true
      (bind _asbp_weapon (cast `/Game/Blueprints/Equipment_System/BP_Weapon` (`.HitActor` (`GameplayStatics.BreakHitResult` _outhit))))
      (`self.AddWeapon` (`/Game/Blueprints/Equipment_System/BP_Weapon.ItemData` _asbp_weapon))
      (`Actor.K2_DestroyActor` _asbp_weapon))))

(event `EnhancedInput|/Game/Input/Actions/IA_EquipmentMenu`
  (params (ActionValue :type Boolean) (ElapsedSeconds :type "Float (double-precision)") (TriggeredSeconds :type "Float (double-precision)") (InputAction :type "InputAction Object Reference" :default "/Game/Input/Actions/IA_EquipmentMenu.IA_EquipmentMenu"))
  ;[0.05098 0.05098 0.05098] Equipment Menu
  (:`Started`
    (if (`self.IsEquipmentMenuOpen`)
      (`self.CloseEquipmentMenu`)
      (else
        (`self.OpenEquipmentMenu`)))))

(event `CloseEquipmentMenu`
  (bind _returnvalue (`GameplayStatics.GetPlayerController` 0))
  ;[0.05098 0.05098 0.05098] Equipment Menu
  (bind _equipmentwidget (`self.EquipmentWidget`)
    (:`then`
      (`Widget.SetVisibility` _equipmentwidget "Hidden")
      (set `self.IsEquipmentMenuOpen` false)
      (set `PlayerController.bShowMouseCursor` false _returnvalue)
      (`WidgetBlueprintLibrary.SetInputMode_GameOnly` _returnvalue)
      (bind _asbp_third_person_character (cast `/Game/Blueprints/Player/BP_ThirdPersonCharacter` (`self.GetOwner`)))
      (`CharacterMovementComponent.SetMovementMode` (`Character.CharacterMovement` _asbp_third_person_character) "MOVE_Walking" 0)
      (set `/Game/Blueprints/Combat/BPC_Attack.CanAttack` true (`/Game/Blueprints/Player/BP_ThirdPersonCharacter.BPC_Attack` _asbp_third_person_character)))
    (:`else`)))

(event `OpenEquipmentMenu`
  (bind _returnvalue (`GameplayStatics.GetPlayerController` 0))
  ;[0.05098 0.05098 0.05098] Equipment Menu
  (bind _equipmentwidget (`self.EquipmentWidget`)
    (:`then`
      _)
    (:`else`
      (bind _returnvalue_2 (`|GenericCreateObject` "/Game/UI/Equipment_System/WB_EquipmentMenu.WB_EquipmentMenu_C"))
      (bind _output_get (set `self.EquipmentWidget` _returnvalue_2))
      (`UserWidget.AddToViewport` _output_get 0)))
  (`Widget.SetVisibility` _equipmentwidget "Visible")
  (set `self.IsEquipmentMenuOpen` true)
  (set `PlayerController.bShowMouseCursor` true _returnvalue)
  (`WidgetBlueprintLibrary.SetInputMode_GameAndUIEx` _returnvalue (`self.EquipmentWidget`))
  (bind _asbp_third_person_character (cast `/Game/Blueprints/Player/BP_ThirdPersonCharacter` (`self.GetOwner`)))
  (`CharacterMovementComponent.SetMovementMode` (`Character.CharacterMovement` _asbp_third_person_character) "MOVE_None" 0)
  (set `/Game/Blueprints/Combat/BPC_Attack.CanAttack` false (`/Game/Blueprints/Player/BP_ThirdPersonCharacter.BPC_Attack` _asbp_third_person_character)))

(fn `AddWeapon`
  (params (NewItem :type "/Game/Blueprints/Equipment_System/S_Slot Structure (by ref)"))
  (`KismetArrayLibrary.Array_Add` (`self.WeaponSlots`) NewItem))